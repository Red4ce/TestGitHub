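; Card slot actor for TokouFight that spawns a scaled-down BP_Card at its own location on BeginPlay and glides it to a destination.
; A Tick gate, opened after spawning, interpolates the card toward GoalDestination and FinalRotation, then closes once location is within tolerance.
; OpenDisplacement ignores its Goal input, and the multi-card hand spacing logic is unconnected.
; An author note says the movement logic belongs on BP_Card.
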(event `self.ReceiveTick`
  (params (DeltaSeconds :type "Float (single-precision)"))
  (bind _goal_destination (`self.Goal Destination`))
  ;[1 1 1] Should be on BP_Card
  (set `self.Delta Time` DeltaSeconds)
  (`/Engine/EditorBlueprintResources/StandardMacros.Gate` true :!label _label
    (:`Exit`
      (bind _returnvalue (`self.K2_GetActorLocation` (stale `Spawn Card` _returnvalue)))
      (`self.K2_SetActorLocationAndRotation` (stale `Spawn Card` _returnvalue) (`KismetMathLibrary.VInterpTo` _returnvalue _goal_destination (`self.Delta Time`) (`self.Interp Speed`)) (`KismetMathLibrary.RInterpTo` (`self.K2_GetActorRotation` (stale `Spawn Card` _returnvalue)) (`self.Final Rotation`) (`self.Delta Time`) (`self.Rotation Interp Speed`)) false false)
      (if (`KismetMathLibrary.NearlyEqual_FloatFloat` (`KismetMathLibrary.VSize` (- _returnvalue _goal_destination)) 0.0 (`self.Error Tolerance`))
        (`KismetSystemLibrary.PrintString` "ARRIVED !!!" true true (struct :`R` 0.143334 :`G` 0.770833 :`A` 1.0))
        (`self.Close Displacement`)
        (else
          (`KismetSystemLibrary.PrintString` "NOT ARRIVED" true true (struct :`R` 0.833333 :`A` 1.0)))))))

(event `Open Displacement`
  (params (Goal :type "Vector Structure"))
  ;[1 1 1] Should be on BP_Card
  (goto _label :!via `Open`))

(event `Close Displacement`
  ;[1 1 1] Should be on BP_Card
  (goto _label :!via `Close`))

(event `Spawn Card`
  (bind (_returnvalue_x _returnvalue_y _returnvalue_z) (`KismetMathLibrary.BreakVector` (`SceneComponent.K2_GetComponentLocation` (`self.DefaultSceneRoot`))))
  (bind _returnvalue (`|SpawnActorFromClass` "/Game/TokouFight/BP_Card.BP_Card_C" (`KismetMathLibrary.MakeTransform` (`KismetMathLibrary.MakeVector` _returnvalue_x _returnvalue_y _returnvalue_z) (struct) (0.15 0.15 0.15)) "Undefined" "OverrideRootScale" null false null :!label _label_2))
  (`self.Open Displacement` (0.0 0.0 0.0)))

(event `self.ReceiveBeginPlay`
  (goto _label_2))

(fn `UserConstructionScript`)