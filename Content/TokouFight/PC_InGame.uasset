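; In-game player controller for TokouFight that binds keyboard shortcuts to card and slot actions.
; B calls the draw card event on GM_InGame, while C and D add and remove slots on the BP_SlotManager found in the level.
; Code to create the DragFrom and in-game screen widgets is present but unconnected, so it never runs.
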(event `self.ReceiveBeginPlay`)

(event `Key|B`
  (params (Key :type "Key Structure"))
  (:`Pressed`
    (`/Game/TokouFight/GM_InGame.DrawCardEvent` (cast `/Game/TokouFight/GM_InGame` (`GameplayStatics.GetGameMode`) :!pure true))))

(event `Key|C`
  (params (Key :type "Key Structure"))
  (:`Pressed`
    (bind _returnvalue (`GameplayStatics.GetActorOfClass` "/Game/TokouFight/BP_SlotManager.BP_SlotManager_C"))
    (`/Game/TokouFight/BP_SlotManager.AddSlot` _returnvalue)))

(event `Key|D`
  (params (Key :type "Key Structure"))
  (:`Pressed`
    (bind _returnvalue (`GameplayStatics.GetActorOfClass` "/Game/TokouFight/BP_SlotManager.BP_SlotManager_C"))
    (`/Game/TokouFight/BP_SlotManager.RemoveSlot` _returnvalue)))

(fn `UserConstructionScript`)