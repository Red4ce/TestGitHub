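; BP_Card is a card actor for TokouFight that glides to a requested location and rotation.
; CardMove opens a gate on Tick, which eases the actor toward the goal with separate movement and rotation interp speeds.
; When the next interpolated location step falls within the error tolerance, CardStop closes the gate; rotation completion is not checked.
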(event `self.ReceiveTick`
  (params (DeltaSeconds :type "Float (single-precision)"))
  (bind _returnvalue (`self.K2_GetActorLocation`))
  (set `self.Delta Time` DeltaSeconds)
  (`/Engine/EditorBlueprintResources/StandardMacros.Gate` true :!label _label
    (:`Exit`
      (bind _returnvalue_2 (`KismetMathLibrary.VInterpTo` _returnvalue (stale `Card Move` `Goal Destination`) (`self.Delta Time`) (`self.Movement Interp Speed`)))
      (`self.K2_SetActorLocationAndRotation` _returnvalue_2 (`KismetMathLibrary.RInterpTo` (`self.K2_GetActorRotation`) (stale `Card Move` `Goal Rotation`) (`self.Delta Time`) (`self.Rotation Interp Speed`)))
      (if (`KismetMathLibrary.NearlyEqual_FloatFloat` (`KismetMathLibrary.VSize` (- _returnvalue _returnvalue_2)) 0.0 (`self.Error Tolerance`))
        (`self.Card Stop`)))))

(event `Card Move`
  (params (`Goal Destination` :type "Vector Structure") (`Goal Rotation` :type "Rotator Structure"))
  (goto _label :!via `Open`))

(event `Card Stop`
  (goto _label :!via `Close`))

(fn `UserConstructionScript`)