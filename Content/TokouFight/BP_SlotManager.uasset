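; BP_SlotManager spawns and tracks BP_CardSlot actors, apparently laying out a hand of cards.
; BeginPlay creates the origin slot; AddSlot chains each next one from the last, stepping position, roll and a cumulative Z drop into a fan.
; UpdateSlotNumber spawns slots in a loop without storing them or setting transforms.
; Work in progress: centering only prints parity, RemoveSlot destroys nothing and leaves CardSlots untouched, and TestCardMove is a debug move.
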(event `UpdateSlotNumber`
  (params (CardsInHand :type "Array of /Game/TokouFight/BP_Card Object Reference") (CardsInHandNUmber :type Integer))
  (bind _output_get (set `self.Cards in Hand Number` CardsInHandNUmber))
  (for _ (range (+ _output_get 1))
    (`|SpawnActorFromClass` "/Game/TokouFight/BP_CardSlot.BP_CardSlot_C" (`KismetMathLibrary.MakeTransform` (0.0 0.0 0.0)) "Undefined" "OverrideRootScale" null null)))

(event `self.ReceiveBeginPlay`
  (bind _returnvalue (`|SpawnActorFromClass` "/Game/TokouFight/BP_CardSlot.BP_CardSlot_C" (`self.OriginSpawn`) "Undefined" "OverrideRootScale" null null))
  (`KismetArrayLibrary.Array_Add` (`self.CardSlots`) _returnvalue))

(event `AddSlot`
  (bind _cardslots (`self.CardSlots`))
  (bind _returnvalue (`|SpawnActorFromClass` "/Game/TokouFight/BP_CardSlot.BP_CardSlot_C" (`self.AddNextSlotTransform` (`|GetArrayItem` _cardslots (`KismetArrayLibrary.Array_LastIndex` _cardslots))) "Undefined" "OverrideRootScale" null null))
  (`KismetArrayLibrary.Array_Add` (`self.CardSlots`) _returnvalue)
  (`self.UpdateCenterCardsPosition`))

(event `RemoveSlot`
  (bind _outactors (`GameplayStatics.GetAllActorsOfClass` "/Game/TokouFight/BP_CardSlot.BP_CardSlot_C"))
  (`KismetArrayLibrary.Array_Remove` _outactors (`KismetArrayLibrary.Array_LastIndex` _outactors))
  (`KismetSystemLibrary.PrintString` (`KismetStringLibrary.Conv_IntToString` (`KismetArrayLibrary.Array_Length` _outactors))))

(event `Test Card Move`
  (bind _outactors (`GameplayStatics.GetAllActorsOfClass` "/Game/TokouFight/BP_Card.BP_Card_C"))
  (`KismetSystemLibrary.PrintString` "Hello")
  (bind _output (`|GetArrayItem` _outactors 5))
  (`/Game/TokouFight/BP_Card.Card Move` (`|GetArrayItem` _outactors) (`self.K2_GetActorLocation` _output) (`self.K2_GetActorRotation` _output)))

(fn `AddNextSlotTransform`
  (params (self2 :type "Actor Object Reference"))
  (returns (TransformToSpawn :type "Transform Structure"))
  (set `self.YOffset` (- (`self.YOffset`) 0.41))
  (return (`KismetMathLibrary.MakeTransform` (`KismetMathLibrary.MakeVector` (+ (.x (.location (`self.GetTransform` self2))) 0.1) (- (.y (.location (`self.GetTransform` self2))) 10.0) (+ (.z (.location (`self.GetTransform` self2))) (`self.YOffset`))) (`KismetMathLibrary.MakeRotator` (- (.roll (.rotation (`self.GetTransform` self2))) 4.5) (.pitch (.rotation (`self.GetTransform` self2))) (.yaw (.rotation (`self.GetTransform` self2)))) (.scale (`self.GetTransform` self2)))))

(fn `UpdateCenterCardsPosition`
  (if (== (mod (+ (`KismetArrayLibrary.Array_LastIndex` (`self.CardSlots`)) 1) 2) 0)
    (`KismetSystemLibrary.PrintString` "PAIR")
    (else
      (`KismetSystemLibrary.PrintString` "IMPAIR"))))

(fn `UserConstructionScript`)